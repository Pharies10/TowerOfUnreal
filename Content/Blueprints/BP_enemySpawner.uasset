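; Enemy spawner Blueprint that populates an area with enemies and clears it as the player crosses its volumes.
; Trigger and Destroyer overlaps by Player-tagged actors both toggle the shared Spawned state.
; Spawning creates set counts of chase and random AI pawns at random points inside the Spawner box and reveals the PathEnemies actors.
; Clearing destroys the tracked pawns and hides the path enemies again, as they are at BeginPlay.
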(event OnComponentBeginOverlap(Trigger)
  (params (OverlappedComponent :type Primitive%20Component%20Object%20Reference) (OtherActor :type Actor%20Object%20Reference) (OtherComp :type Primitive%20Component%20Object%20Reference) (OtherBodyIndex :type Integer) (bFromSweep :type Boolean) (SweepResult :type Hit%20Result%20Structure%20%28by%20ref%29))
  (if (Actor|ActorHasTag OtherActor "Player")
    (if (not (Variables|Default|Getspawned))
      (CallFunction|BeginSpawn)
      (Variables|Default|Setspawned true)
      (else
        (CallFunction|DestroyEnemy)
        (Variables|Default|Setspawned false)))))

(event OnComponentBeginOverlap(Destroyer)
  (params (OverlappedComponent :type Primitive%20Component%20Object%20Reference) (OtherActor :type Actor%20Object%20Reference) (OtherComp :type Primitive%20Component%20Object%20Reference) (OtherBodyIndex :type Integer) (bFromSweep :type Boolean) (SweepResult :type Hit%20Result%20Structure%20%28by%20ref%29))
  (if (Actor|ActorHasTag OtherActor "Player")
    (if (Variables|Default|Getspawned)
      (CallFunction|DestroyEnemy)
      (Variables|Default|Setspawned false)
      (else
        (CallFunction|BeginSpawn)
        (Variables|Default|Setspawned true)))))

(event Custom|spawnEnemys
  (params (TypeOfEnemy :type Pawn%20Class%20Reference))
  (bind _spawner (Variables|Default|GetSpawner))
  (bind _returnvalue (AI|SpawnAIFromClass TypeOfEnemy 0 (Math|Random|RandomPointinBoundingBox (Transformation|GetWorldLocation _spawner) (Components|Box|GetScaledBoxExtent _spawner)) "0, 0, 0" false))
  (if (Utilities|IsValid _returnvalue)
    (Utilities|Array|Add (Variables|Default|GetEnemiesSpawned) _returnvalue)))

(event Custom|beginSpawn
  (Utilities|FlowControl|Sequence
    (:then_0
      (for _index (range 0 (- (Variables|Default|GetenemyChasetoSpawn) 1))
        (CallFunction|SpawnEnemys "/Game/AIStuff/EnemyChase.EnemyChase_C")))
    (:then_1
      (for _index_2 (range 0 (- (Variables|Default|GetenemyRandomtoSpawn) 1))
        (CallFunction|SpawnEnemys "/Game/AIStuff/EnemyRandom.EnemyRandom_C")))
    (:then_2
      (for _array_element (Variables|Default|GetpathEnemies)
        (Rendering|SetActorHiddenInGame _array_element false)))))

(event Custom|destroyEnemy
  (bind _enemiesspawned (Variables|Default|GetEnemiesSpawned))
  (Utilities|FlowControl|Sequence
    (:then_0
      (for _array_element _enemiesspawned
        (Actor|DestroyActor _array_element))
      (Utilities|Array|Clear _enemiesspawned))
    (:then_1
      (for _array_element_2 (Variables|Default|GetpathEnemies)
        (Rendering|SetActorHiddenInGame _array_element_2 true)))))

(event EventBeginPlay
  (for _array_element (Variables|Default|GetpathEnemies)
    (Rendering|SetActorHiddenInGame _array_element true)))

(fn ConstructionScript)