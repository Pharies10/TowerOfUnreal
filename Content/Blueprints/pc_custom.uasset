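; Custom player controller Blueprint that toggles the pause menu when the pause input action is pressed.
; Pausing creates and shows a PauseMenu widget, switches to game-and-UI input, shows the mouse cursor and pauses the game.
; Unpausing finds PauseMenu widgets by class to remove them, restores game-only input, hides the cursor and resumes play, tracked by an IsPaused flag.
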(event Input|ActionEvents|InputActionpause
  (params (Key :type Key%20Structure :default "None"))
  (bind _returnvalue (Game|GetPlayerController 0))
  (bind _returnvalue_2 (Game|GetPlayerController 0))
  (:Pressed
    (if (Variables|Default|GetisPaused)
      (bind _foundwidgets (Widget|GetAllWidgetsOfClass "/Game/Widgets/pauseMenu.pauseMenu_C" false))
      (Widget|RemovefromParent _foundwidgets)
      (Input|SetInputModeGameOnly _returnvalue)
      (Variables|/Script/Engine.PlayerController|SetbShowMouseCursor _returnvalue false)
      (Game|SetGamePaused false)
      (Variables|Default|SetisPaused false)
      (else
        (bind _returnvalue_3 (UserInterface|CreateWidget "/Game/Widgets/pauseMenu.pauseMenu_C"))
        (UserInterface|Viewport|AddtoViewport _returnvalue_3 0)
        (Input|SetInputModeGameandUI _returnvalue_2 0 "DoNotLock" true)
        (Variables|/Script/Engine.PlayerController|SetbShowMouseCursor _returnvalue_2 true)
        (Game|SetGamePaused true)
        (Variables|Default|SetisPaused true)))))

(fn ConstructionScript)